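; BP_Player is a third-person player character with Enhanced Input movement, camera look, a toggleable rifle and aiming.
; Equipping toggles the rifle's visibility after a short delay, while an aim timeline shortens and raises the spring arm, reversing on release.
; Holding fire with the rifle equipped loops a timer that plays the fire montage, whose notify triggers a debug-drawn muzzle line trace with no hit handling.
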(event Custom|Fire%20Rifle
  (bind _rifle (Variables|Default|GetRifle))
  (bind _returnvalue (Transformation|GetSocketTransform _rifle "Muzzle" "RTS_World"))
  ;[0.1346 0.1986 0.2344] Fire
  (Animation|Montage|PlayMontage (Variables|Character|GetMesh) "/Game/Characters/Animations/Rifle/Fire_Rifle_Montage.Fire_Rifle_Montage"
    (:OnNotifyBegin
      ;;[0.1346 0.1986 0.2344] Line Ray from bullet
      (Collision|LineTraceByChannel (.location _returnvalue) (+ (.location _returnvalue) (* (Math|Vector|GetForwardVector (.rotation _returnvalue)) 5e+03)) "TraceTypeQuery1" false 0 "ForDuration"))))

(event Input|EnhancedActionEvents|EnhancedInputActionIA_Move
  (params (ActionValue :type Vector%202D%20Structure) (ElapsedSeconds :type Float%20%28double-precision%29) (TriggeredSeconds :type Float%20%28double-precision%29) (InputAction :type Input%20Action%20Object%20Reference :default "/Game/Input/IA_Move.IA_Move"))
  (bind _returnvalue (Pawn|GetControlRotation :!class /Script/Engine.Pawn))
  (bind _returnvalue_2 (Pawn|GetControlRotation :!class /Script/Engine.Pawn))
  ;[0.1346 0.1986 0.2344] Movement And Camera Look
  (Pawn|Input|AddMovementInput (Math|Vector|GetRightVector (Math|Rotator|MakeRotator (.roll _returnvalue) 0.0 (.yaw _returnvalue))) (.x ActionValue) false)
  (Pawn|Input|AddMovementInput (Math|Vector|GetForwardVector (Math|Rotator|MakeRotator (.roll _returnvalue_2) 0.0 (.yaw _returnvalue_2))) (.y ActionValue) false))

(event Input|EnhancedActionEvents|EnhancedInputActionIA_Look
  (params (ActionValue :type Vector%202D%20Structure) (ElapsedSeconds :type Float%20%28double-precision%29) (TriggeredSeconds :type Float%20%28double-precision%29) (InputAction :type Input%20Action%20Object%20Reference :default "/Game/Input/IA_Look.IA_Look"))
  ;[0.1346 0.1986 0.2344] Movement And Camera Look
  (Pawn|Input|AddControllerYawInput (.x ActionValue))
  (Pawn|Input|AddControllerPitchInput (* (.y ActionValue) -1.0)))

(event Input|EnhancedActionEvents|EnhancedInputActionIA_EquipRifle
  (params (ActionValue :type Boolean) (ElapsedSeconds :type Float%20%28double-precision%29) (TriggeredSeconds :type Float%20%28double-precision%29) (InputAction :type Input%20Action%20Object%20Reference :default "/Game/Input/IA_EquipRifle.IA_EquipRifle"))
  ;[0.1346 0.1986 0.2344] Equip and Unequip Rifle
  (:Started
    (if (not (Variables|Default|GetRifle%20Equiped))
      (Variables|Default|SetRifle%20Equiped true)
      (Utilities|FlowControl|Delay 0.8)
      (Rendering|SetVisibility (Variables|Default|GetRifle) true false)
      (else
        (Variables|Default|SetRifle%20Equiped false)
        (Utilities|FlowControl|Delay 0.8)
        (Rendering|SetVisibility (Variables|Default|GetRifle) false false)))))

(event Input|EnhancedActionEvents|EnhancedInputActionIA_Aim
  (params (ActionValue :type Boolean) (ElapsedSeconds :type Float%20%28double-precision%29) (TriggeredSeconds :type Float%20%28double-precision%29) (InputAction :type Input%20Action%20Object%20Reference :default "/Game/Input/IA_Aim.IA_Aim"))
  (bind _springarm (Variables|Default|GetSpringArm))
  ;[0.1346 0.1986 0.2344] Aiming
  (:Started
    (Variables|Default|SetIs%20Aiming true)
    (bind _arm_length (Timeline|Aim Play)
      (:Update
        (Variables|/Script/Engine.SpringArmComponent|SetTargetArmLength (Variables|Default|GetSpringArm) (Math|Float|Lerp 3e+02 1.5e+02 _arm_length))
        (Variables|/Script/Engine.SpringArmComponent|SetSocketOffset _springarm (Math|Vector|MakeVector (.x (Variables|/Script/Engine.SpringArmComponent|GetSocketOffset _springarm)) (.y (Variables|/Script/Engine.SpringArmComponent|GetSocketOffset _springarm)) (Math|Float|Lerp 0.0 25.0 _arm_length))))))
  (:Completed
    (Variables|Default|SetIs%20Aiming false)
    (Timeline|Aim Reverse)))

(event Input|EnhancedActionEvents|EnhancedInputActionIA_Fire
  (params (ActionValue :type Boolean) (ElapsedSeconds :type Float%20%28double-precision%29) (TriggeredSeconds :type Float%20%28double-precision%29) (InputAction :type Input%20Action%20Object%20Reference :default "/Game/Input/IA_Fire.IA_Fire"))
  ;[0.1346 0.1986 0.2344] Fire
  (:Started
    (if (Variables|Default|GetRifle%20Equiped)
      (bind _returnvalue (Utilities|Time|SetTimerbyEvent (delegate Custom|Fire%20Rifle) 0.1 true))))
  (:Completed
    (Utilities|Time|ClearandInvalidateTimerbyHandle _returnvalue)))

(event EventBeginPlay
  ;[0.1346 0.1986 0.2344] Add Input
  (Input|AddMappingContext (PlayerController|LocalPlayerSubsystems|GetEnhancedInputLocalPlayerSubsystem (Game|GetPlayerController 0)) "/Game/Input/IMC_PlayerInput.IMC_PlayerInput" 0 "(bIgnoreAllPressedKeysUntilRelease=True,bForceImmediately=False,bNotifyUserSettings=False)"))

(fn ConstructionScript)