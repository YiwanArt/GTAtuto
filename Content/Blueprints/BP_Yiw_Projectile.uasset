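; BP_Yiw_Projectile is an arrow projectile actor that deals damage on impact.
; On BeginPlay, it assigns the arrow Niagara effect once the player pawn casts successfully to BP_Player.
; When its Box component hits, it spawns a pooled Niagara hit effect, destroys itself and applies fixed damage to the hit actor.
; Actors tagged "Character" also get a blood splat emitter oriented along the hit normal.
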(event OnComponentHit(Box)
  (params (HitComponent :type Primitive%20Component%20Object%20Reference) (OtherActor :type Actor%20Object%20Reference) (OtherComp :type Primitive%20Component%20Object%20Reference) (NormalImpulse :type Vector :default "0, 0, 0") (Hit :type Hit%20Result%20Structure%20%28by%20ref%29))
  (bind (_bblockinghit _binitialoverlap _time _distance _location _impactpoint _normal _impactnormal _physmat _hitactor) (Collision|BreakHitResult Hit))
  (Niagara|SpawnSystematLocation (Variables|Default|GetNiagaraHit) _location "0, 0, 0" "1.000000,1.000000,1.000000" true true "AutoRelease")
  (Actor|DestroyActor)
  (Game|Damage|ApplyDamage _hitactor 1e+01 0 0)
  (if (Actor|ActorHasTag _hitactor "Character")
    (Effects|SpawnEmitteratLocation "/Game/Realistic_Starter_VFX_Pack_Vol2/Particles/Blood/P_Blood_Splat_Cone.P_Blood_Splat_Cone" _impactpoint (Math|Rotator|MakeRotfromX _normal) "0.700000,0.700000,0.300000")))

(event EventBeginPlay
  (Utilities|Casting|CastToBP_Player (Game|Player|GetPlayerPawn 0))
  (Class|NiagaraComponent|SetAsset (Variables|Default|GetNiagara) (Variables|Default|GetNiagaraArrow) true))

(fn ConstructionScript)